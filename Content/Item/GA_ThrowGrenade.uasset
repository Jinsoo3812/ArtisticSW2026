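; GA_ThrowGrenade is a gameplay ability that lets the Attacker aim and throw a grenade.
; On activation, a looping timer repeatedly predicts the projectile path from the control rotation and starts a WaitInputRelease task on each tick.
; On release, it clears the timer, spawns BP_GrenadeProjectile ahead of the avatar facing the control rotation, consumes the equipped item and ends the ability.
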(event `self.K2_ActivateAbility`
  (bind _returnvalue (`KismetSystemLibrary.K2_SetTimerDelegate` (delegate `DrawTrajectory`) 0.02 true))
  (set `self.DrawTimerHandle` _returnvalue))

(event `DrawTrajectory`
  (bind _returnvalue (`self.GetAvatarActorFromActorInfo`))
  (bind _asattacker (cast `Attacker` _returnvalue :!pure true))
  (bind _returnvalue_2 (`Pawn.GetControlRotation` _asattacker))
  (bind _returnvalue_3 (`KismetMathLibrary.GetForwardVector` _returnvalue_2))
  (`GameplayStatics.Blueprint_PredictProjectilePath_ByTraceChannel` (+ (* _returnvalue_3 40.0) (+ (`Actor.K2_GetActorLocation` _asattacker) (0.0 0.0 50.0))) (* _returnvalue_3 1000.0) true 15.0 "ECC_Camera" false (`|MakeArray` _returnvalue) "ForOneFrame")
  (`AbilityTask_WaitInputRelease.WaitInputRelease` false
    (:`OnRelease`
      (`KismetSystemLibrary.K2_ClearAndInvalidateTimerHandle` (`self.DrawTimerHandle`))
      (`|SpawnActorFromClass` "/Game/Item/BP_GrenadeProjectile.BP_GrenadeProjectile_C" (`KismetMathLibrary.MakeTransform` (+ (+ (`Actor.K2_GetActorLocation` _returnvalue) (0.0 0.0 50.0)) (* (`Actor.GetActorForwardVector` _returnvalue) 80.0)) _returnvalue_2) "AlwaysSpawn" "MultiplyWithRoot" null null)
      (bind _asattacker_2 (cast `Attacker` _returnvalue))
      (`Attacker.ConsumeEquippedItem` _asattacker_2)
      (`self.K2_EndAbility`))))