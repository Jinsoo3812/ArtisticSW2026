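; BP_SpawnSmokeGrenade is a spawner actor from the Shooter VFX pack that repeatedly spawns smoke grenades at its own transform.
; After an initial delay on BeginPlay, it spawns one grenade immediately and starts a looping timer for further spawns.
; The Version01 flag selects between M_SmokeGrenade_01 and M_SmokeGrenade_02, with only the second receiving the Effect setting.
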(event `Again`
  (bind _returnvalue (`self.GetTransform`))
  (if (`self.Version01`) :!label _label
    (`|SpawnActorFromClass` "/Game/Resources_Assets/Shooter_VFXPack/Blueprints/M_SmokeGrenade_01.M_SmokeGrenade_01_C" _returnvalue "Undefined" "OverrideRootScale" null null)
    (else
      (`|SpawnActorFromClass` "/Game/Resources_Assets/Shooter_VFXPack/Blueprints/M_SmokeGrenade_02.M_SmokeGrenade_02_C" _returnvalue "Undefined" "OverrideRootScale" null (`self.Effect`) null))))

(event `self.ReceiveBeginPlay`
  (`KismetSystemLibrary.Delay` (`self.InitialDelay`))
  (`|ExecutionSequence`
    (:`then_0`
      (`KismetSystemLibrary.K2_SetTimerDelegate` (delegate `Again`) (`self.Delay`) true))
    (:`then_1`
      (goto _label))))

(fn `UserConstructionScript`)