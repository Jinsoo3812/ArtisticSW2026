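; Base Gameplay Ability for enemy melee attacks, which plays an attack montage on the owning BP_BaseEnemy.
; Gameplay events for scan start and end open and close the current weapon's hit scan during the montage.
; The start event passes the weapon a damage effect spec with SetByCaller magnitude.
; The ability ends when the montage completes, is interrupted or is cancelled, and OnEndAbility also stops the hit scan.
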(event `self.K2_ActivateAbility`
  (bind _returnvalue (`self.GetAvatarActorFromActorInfo`))
  (`/Engine/EditorBlueprintResources/StandardMacros.IsValid` _returnvalue
    (:`Is Valid`
      (bind _asbp_my_enemy (cast `/Game/GameplayAbilitySystem/Enemy/BP_BaseEnemy` _returnvalue))
      (set `self.MyEnemy` _asbp_my_enemy)
      (`AbilityTask_PlayMontageAndWait.CreatePlayMontageAndWaitProxy` "None" "/Game/GameplayAbilitySystem/Character/AnimMontage/AM_Attack01.AM_Attack01" 1.0 "None" true 1.0 0.0 true
        (:`then`
          (`AbilityTask_WaitGameplayEvent.WaitGameplayEvent` (struct :`TagName` "Event.HandleScan.Start") null true
            (:`then`
              (`AbilityTask_WaitGameplayEvent.WaitGameplayEvent` (struct :`TagName` "Event.HandleScan.End") null true
                (:`EventReceived`
                  (`self.HandleHitScanEnd`))))
            (:`EventReceived`
              (`self.HandleHitScanStart`))))
        (:`OnCompleted`
          (`self.K2_EndAbility` :!label _label))
        (:`OnInterrupted`
          (goto _label))
        (:`OnCancelled`
          (goto _label))))
    (:`Is Not Valid`
      (`self.K2_EndAbility`))))

(event `HandleHitScanStart`
  (bind _returnvalue (`AbilitySystemBlueprintLibrary.AssignTagSetByCallerMagnitude` (`self.MakeOutgoingGameplayEffectSpec` (`self.DamageEffectClass`)) (struct :`TagName` "Data.Damage") (`self.DamageMagnitude`)))
  (`BaseWeapon.HitScanStart` (`BaseWeaponComponent.GetCurrentWeapon` (`Actor.GetComponentByClass` (`self.MyEnemy`) "/Script/Enemy.BaseWeaponComponent")) _returnvalue))

(event `HandleHitScanEnd`
  (`BaseWeapon.HitScanEnd` (`BaseWeaponComponent.GetCurrentWeapon` (`Actor.GetComponentByClass` (`self.MyEnemy`) "/Script/Enemy.BaseWeaponComponent"))))

(event `self.K2_OnEndAbility`
  (params (bWasCancelled :type Boolean))
  (`BaseWeapon.HitScanEnd` (`BaseWeaponComponent.GetCurrentWeapon` (`Actor.GetComponentByClass` (`self.MyEnemy`) "/Script/Enemy.BaseWeaponComponent"))))